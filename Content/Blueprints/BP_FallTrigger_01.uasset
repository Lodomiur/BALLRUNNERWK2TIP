(event `self.Box.OnComponentEndOverlap`
  (params (OverlappedComponent :type "PrimitiveComponent Object Reference") (OtherActor :type "Actor Object Reference") (OtherComp :type "PrimitiveComponent Object Reference") (OtherBodyIndex :type Integer))
  (bind _returnvalue (`GameplayStatics.GetCurrentLevelName` true))
  ;[1 1 1] fade camera
  (`PlayerCameraManager.StartCameraFade` (`PlayerController.PlayerCameraManager` (`GameplayStatics.GetPlayerController` 0)) 0.0 1.0 1.0 (struct :`A` 1.0) false false)
  (`KismetSystemLibrary.Delay` 2.0)
  (`GameplayStatics.OpenLevel` (`KismetStringLibrary.Conv_StringToName` _returnvalue))
  (`KismetSystemLibrary.PrintString` "Przegrales zagraj jeszcze raz" true true (struct :`R` 1.0 :`B` 0.009844 :`A` 1.0) 5.0))

(event `self.ReceiveBeginPlay`
  ;[1 1 1] FADE W DRUGA STRONE
  (`PlayerCameraManager.StartCameraFade` (`PlayerController.PlayerCameraManager` (`GameplayStatics.GetPlayerController` 0)) 1.0 0.0 1.0 (struct :`R` 1.0 :`B` 0.020907 :`A` 1.0) false false))

(fn `UserConstructionScript`)